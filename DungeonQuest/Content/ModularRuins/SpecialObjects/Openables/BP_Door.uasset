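; BP_Door is an openable double door that swings its left and right leaves in opposite directions.
; Open/Close toggles IsOpen, plays the matching sound, switches the action label between Open and Close, and plays or reverses the DoorsOpen timeline at a rate set by open or close time.
; The timeline lerps both leaves' yaw, and OnReset snaps open doors shut and calls the parent reset.
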(event `self.K2_OnReset`
  (if (`self.isOpen`)
    (set `self.isOpen` false)
    (`|ExecutionSequence`
      (:`then_0`
        (`SceneComponent.K2_SetRelativeRotation` (`self.DoorRight`) (`KismetMathLibrary.MakeRotator` 0.0) false false))
      (:`then_1`
        (`SceneComponent.K2_SetRelativeRotation` (`self.DoorLeft`) (`KismetMathLibrary.MakeRotator` 0.0) false false))
      (:`then_2`
        (`parent.K2_OnReset`)
        (bind (_direction _doors) (`Timeline|DoorsOpen` :!via `SetNewTime` :!label _label)
          (:`Update`
            (`|ExecutionSequence`
              (:`then_0`
                (`SceneComponent.K2_SetRelativeRotation` (`self.DoorRight`) (`KismetMathLibrary.MakeRotator` 0.0 0.0 (`KismetMathLibrary.Lerp` 0.0 -109.0 _doors)) false false))
              (:`then_1`
                (`SceneComponent.K2_SetRelativeRotation` (`self.DoorLeft`) (`KismetMathLibrary.MakeRotator` 0.0 0.0 (`KismetMathLibrary.Lerp` 0.0 109.0 _doors)) false false)))))))))

(event `self.Open/Close`
  (if (`self.isOpen`)
    (`TimelineComponent.SetPlayRate` (`self.DoorsOpen`) (/ 1.0 (`self.timeToClose`)))
    (set `self.isOpen` false)
    (`GameplayStatics.PlaySound2D` "/Game/Audio/Objects/Door/doorClose_2.doorClose_2" 1.0 1.0 0.0 null null)
    (`self.SetActionType` "Open")
    (goto _label :!via `Reverse`)
    (else
      (`TimelineComponent.SetPlayRate` (`self.DoorsOpen`) (/ 1.0 (`self.timeToOpen`)))
      (set `self.isOpen` true)
      (`GameplayStatics.PlaySound2D` "/Game/Audio/Objects/Door/doorOpen_2.doorOpen_2" 1.0 1.0 0.0 null null)
      (`self.SetActionType` "Close")
      (goto _label))))

(fn `UserConstructionScript`
  (`parent.UserConstructionScript`))