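; BP_Chest is an openable chest whose lid swings open and shut through the Open/Close event.
; Each toggle plays a 2D sound, flips IsOpen, sets the Open or Close action label, and plays or reverses the ChestOpen timeline that rotates the lid's roll.
; On reset, an open chest snaps its lid shut, calls the parent's reset and sets a new timeline time.
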(event `self.K2_OnReset`
  (if (`self.isOpen`)
    (set `self.isOpen` false)
    (`|ExecutionSequence`
      (:`then_0`
        (`SceneComponent.K2_SetRelativeRotation` (`self.ChestLid`) (`KismetMathLibrary.MakeRotator` 0.0 0.0 180.0) false false))
      (:`then_1`
        (`parent.K2_OnReset`)
        (bind (_direction _doors) (`Timeline|ChestOpen` :!via `SetNewTime` :!label _label)
          (:`Update`
            (`SceneComponent.K2_SetRelativeRotation` (`self.ChestLid`) (`KismetMathLibrary.MakeRotator` (`KismetMathLibrary.Lerp` 0.0 90.0 _doors) 0.0 180.0) false false)))))))

(event `self.Open/Close`
  (if (`self.isOpen`)
    (`GameplayStatics.PlaySound2D` "/Game/Audio/Objects/Chest/ChestClose.ChestClose" 1.0 1.0 0.0 null null)
    (set `self.isOpen` false)
    (`self.SetActionType` "Open")
    (goto _label :!via `Reverse`)
    (else
      (`GameplayStatics.PlaySound2D` "/Game/Audio/Objects/Chest/ChestOpen.ChestOpen" 1.0 1.0 0.0 null null)
      (set `self.isOpen` true)
      (`self.SetActionType` "Close")
      (goto _label :!via `PlayFromStart`))))

(fn `UserConstructionScript`
  (`parent.UserConstructionScript`))