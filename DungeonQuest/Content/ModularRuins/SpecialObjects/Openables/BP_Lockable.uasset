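; BP_Lockable is the logic for openable objects that can be locked until the player holds a matching key.
; On interaction it unlocks, with a sound, if the third-person character's picked-up keys contain UnlockKey, or calls Open/Close when already unlocked.
; The action type shows Unlock or Open to match the lock state, and reset re-locks objects with a valid key reference.
; Open/Close is empty here.
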(event `self.K2_OnReset`
  (if (`KismetSystemLibrary.IsValidSoftObjectReference` (`self.unlockKey`))
    (`self.SetActionType` "Unlock")
    (set `self.isLocked` true)
    (else
      (`self.SetActionType` "Open"))))

(event `self.ReceiveBeginPlay`
  (if (`self.isLocked`)
    (`self.SetActionType` "Unlock")
    (else
      (`self.SetActionType` "Open")))
  (`parent.ReceiveBeginPlay`))

(event `self.InteractWith`
  (bind _asbp_third_person_character (cast `/Game/ThirdPerson/Blueprints/BP_ThirdPersonCharacter` (`GameplayStatics.GetPlayerCharacter` 0)))
  (if (`self.isLocked`)
    (if (`KismetArrayLibrary.Array_Contains` (`/Game/ThirdPerson/Blueprints/BP_ThirdPersonCharacter.PickedUpKeys` _asbp_third_person_character) (`self.unlockKey`))
      (`self.Unlock`))
    (else
      (`self.Open/Close`))))

(event `Unlock`
  (set `self.isLocked` false)
  (`GameplayStatics.PlaySound2D` "/Game/Audio/Objects/Lock/mixkit-gear-metallic-lock-sound-2858.mixkit-gear-metallic-lock-sound-2858" 1.0 1.0 0.0 null null)
  (`self.SetActionType` "Open"))

(event `Open/Close`)

(fn `UserConstructionScript`
  (`parent.UserConstructionScript`))