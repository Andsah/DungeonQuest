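; BP_Key is an interactable key pickup that records itself as collected and can be reset.
; Interacting adds it to the game mode's key storage and the player character's picked-up keys, plays a pickup sound, hides its widget and mesh, and moves the actor away.
; ResetKey re-shows the mesh and returns the actor to the transform cached at BeginPlay, without re-showing the widget.
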(event `ResetKey`
  (`SceneComponent.SetVisibility` (`self.Key`) true false)
  (`self.K2_SetActorTransform` (`self.OriginalTransform`)))

(event `self.ReceiveBeginPlay`
  (`parent.ReceiveBeginPlay`)
  (set `self.OriginalTransform` (`self.GetTransform`)))

(event `self.InteractWith`
  (`|ExecutionSequence`
    (:`then_0`
      (bind _asbp_third_person_game_mode (cast `/Game/ThirdPerson/Blueprints/BP_ThirdPersonGameMode` (`GameplayStatics.GetGameMode`)))
      (`KismetArrayLibrary.Array_AddUnique` (`/Game/ThirdPerson/Blueprints/BP_ThirdPersonGameMode.PickedUpKeysStorage` _asbp_third_person_game_mode) self)
      (`GameplayStatics.PlaySound2D` "/Game/Audio/Objects/Lock/KeyPickup.KeyPickup" 1.0 1.0 0.0 null null)
      (`SceneComponent.SetHiddenInGame` (`self.Widget`) true false))
    (:`then_1`
      (bind _asbp_third_person_character (cast `/Game/ThirdPerson/Blueprints/BP_ThirdPersonCharacter` (`GameplayStatics.GetPlayerCharacter` 0)))
      (`KismetArrayLibrary.Array_AddUnique` (`/Game/ThirdPerson/Blueprints/BP_ThirdPersonCharacter.PickedUpKeys` _asbp_third_person_character) (`|ConvertAsset` self))
      (`SceneComponent.SetVisibility` (`self.Key`) false false)
      (`self.K2_SetActorTransform` (`KismetMathLibrary.MakeTransform` (0.0 0.0 0.0))))))

(fn `UserConstructionScript`
  (`parent.UserConstructionScript`))