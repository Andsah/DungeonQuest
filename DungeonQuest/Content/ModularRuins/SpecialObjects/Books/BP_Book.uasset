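; BP_Book is an interactable book that the player opens to read its title and contents on screen.
; Interactwith plays a sound, swaps the closed mesh for the open one, and spawns a TextReaderWidget that receives the text and a reference back to the book.
; It also switches to UI-only input with a cursor and removes the stamina, health and crosshair widgets.
; CloseBook plays a sound and restores the closed mesh.
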(event `CloseBook`
  (`GameplayStatics.PlaySound2D` "/Game/Audio/UI/BookClose.BookClose" 1.0 1.0 0.0 null null)
  (`SceneComponent.SetVisibility` (`self.BookOpen`) false false)
  (`SceneComponent.SetVisibility` (`self.BookClosed`) true false))

(event `self.InteractWith`
  (bind _returnvalue (`GameplayStatics.GetPlayerController` 0))
  (`GameplayStatics.PlaySound2D` "/Game/Audio/UI/BookOpen.BookOpen" 1.0 1.0 0.0 null null)
  (`SceneComponent.SetVisibility` (`self.BookOpen`) true false)
  (`SceneComponent.SetVisibility` (`self.BookClosed`) false false)
  (bind _returnvalue_2 (`|CreateWidget` "/Game/UI/Player/TextReaderWidget.TextReaderWidget_C"))
  (set `/Game/UI/Player/TextReaderWidget.ReadingText` (`self.Contents`) _returnvalue_2)
  (set `/Game/UI/Player/TextReaderWidget.Title` (`self.Title`) _returnvalue_2)
  (set `/Game/UI/Player/TextReaderWidget.OwningBook` self _returnvalue_2)
  (`UserWidget.AddToViewport` _returnvalue_2 0)
  (`WidgetBlueprintLibrary.SetInputMode_UIOnlyEx` _returnvalue _returnvalue_2)
  (set `PlayerController.bShowMouseCursor` true _returnvalue)
  (bind _asbp_third_person_character (cast `/Game/ThirdPerson/Blueprints/BP_ThirdPersonCharacter` (`GameplayStatics.GetPlayerCharacter` 0)))
  (`Widget.RemoveFromParent` (`/Game/ThirdPerson/Blueprints/BP_ThirdPersonCharacter.staminaWidgetRef` _asbp_third_person_character))
  (`Widget.RemoveFromParent` (`/Game/ThirdPerson/Blueprints/BP_ThirdPersonCharacter.healthWidgetREF` _asbp_third_person_character))
  (`Widget.RemoveFromParent` (`/Game/ThirdPerson/Blueprints/BP_ThirdPersonCharacter.CrosshairREF` _asbp_third_person_character)))

(fn `UserConstructionScript`
  (`parent.UserConstructionScript`))