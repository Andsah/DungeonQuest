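; BP_Consumable is a one-use interactable potion, with an empty Consume event as the hook for its effect.
; DisplayPrompt and HidePrompt toggle the widget prompt only while it is unconsumed.
; Interacting plays the drink sound, calls Consume, then flags it consumed and zeroes the mesh's Visibility material parameter.
; Only if a save named after the level exists, it hides the prompt and registers itself in the GameMode's consumed-consumables storage.
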(event `self.DisplayPrompt`
  (`self.NotConsumedYet`
    (:`Out`
      (`SceneComponent.SetHiddenInGame` (`self.Widget`) false false))))

(event `self.HidePrompt`
  (`self.NotConsumedYet`
    (:`Out`
      (`SceneComponent.SetHiddenInGame` (`self.Widget`) true false))))

(event `Consume`)

(event `self.InteractWith`
  (if (not (`self.isConsumed`))
    (`GameplayStatics.PlaySound2D` "/Game/Audio/Objects/Consumable/PotionDrink.PotionDrink" 1.0 1.0 0.0 null null)
    (`self.Consume`)
    (`self.SetConsumed`)
    (bind _returnvalue (`GameplayStatics.GetCurrentLevelName` true))
    (bind _returnvalue_2 (`GameplayStatics.DoesSaveGameExist` _returnvalue))
    (if _returnvalue_2
      (bind _asbp_third_person_game_mode (cast `/Game/ThirdPerson/Blueprints/BP_ThirdPersonGameMode` (`GameplayStatics.GetGameMode`)))
      (`SceneComponent.SetHiddenInGame` (`self.Widget`) true false)
      (`KismetArrayLibrary.Array_AddUnique` (`/Game/ThirdPerson/Blueprints/BP_ThirdPersonGameMode.ConsumedConsumablesStorage` _asbp_third_person_game_mode) self))))

(fn `SetConsumed`
  (set `self.isConsumed` true)
  (`MeshComponent.SetScalarParameterValueOnMaterials` (`self.Base_mesh`) "Visibility" 0.0))

(fn `UserConstructionScript`
  (`parent.UserConstructionScript`))