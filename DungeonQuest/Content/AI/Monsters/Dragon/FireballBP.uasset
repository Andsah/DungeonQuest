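; FireballBP is a dragon fireball projectile aimed at the player.
; On BeginPlay it sets its projectile movement velocity along the normalized direction to the first player character, scaled by ProjectileSpeed, without homing afterward.
; The velocity is passed through SetVelocityInLocalSpace although the direction is computed in world space.
; Overlapping a BP_ThirdPersonCharacter applies Damage and destroys the fireball.
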(event `self.ReceiveBeginPlay`
  (`ProjectileMovementComponent.SetVelocityInLocalSpace` (`self.ProjectileMovement`) (* (`KismetMathLibrary.Normal` (- (`self.K2_GetActorLocation` (`GameplayStatics.GetPlayerCharacter` 0)) (`self.K2_GetActorLocation`))) (`self.ProjectileSpeed`))))

(event `self.ReceiveActorBeginOverlap`
  (params (OtherActor :type "Actor Object Reference"))
  (bind _asbp_third_person_character (cast `/Game/ThirdPerson/Blueprints/BP_ThirdPersonCharacter` OtherActor))
  (`GameplayStatics.ApplyDamage` _asbp_third_person_character (`self.Damage`))
  (`self.K2_DestroyActor`))

(fn `UserConstructionScript`)