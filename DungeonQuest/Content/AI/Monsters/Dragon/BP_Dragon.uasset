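; Dragon monster Blueprint that runs a timed, telegraphed attack pattern when it sees a pawn.
; While alive, PawnSensing flags the player as seen and starts the pattern, with a delayed InAttackPattern gate preventing retriggers.
; The pattern faces the player, briefly switches on an isCharging material parameter as a wind-up, then opens a timed CanAttack window.
; The attack itself is not performed in this graph, which only sets that flag.
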(event `self.PawnSensing.OnSeePawn`
  (params (Pawn :type "Pawn Object Reference"))
  (if (not (`self.isDead`))
    (set `self.isSeeingPlayer` true)
    (if (not (`self.inAttackPattern`))
      (set `self.inAttackPattern` true)
      (`self.AttackPattern`)
      (`KismetSystemLibrary.Delay` 3.5)
      (set `self.inAttackPattern` false))))

(event `self.AttackPattern`
  (bind _mesh (`self.Mesh`))
  (`self.FacePlayer`)
  (`MeshComponent.SetScalarParameterValueOnMaterials` _mesh "isCharging" 1.0)
  (`KismetSystemLibrary.Delay` 0.4)
  (`MeshComponent.SetScalarParameterValueOnMaterials` _mesh "isCharging" 0.0)
  (set `self.canAttack` true)
  (`KismetSystemLibrary.Delay` 1.4)
  (set `self.canAttack` false))

(fn `UserConstructionScript`
  (`parent.UserConstructionScript`))