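; BP_Skeleton is a skeleton monster Blueprint that times a two-hit attack pattern.
; Its AttackPattern event chains delays to alternate wind-up phases with windows where CanAttack is true, the second wind-up lasting longer.
; An isCharging scalar parameter on the mesh materials is switched on during each wind-up and off when the attack window opens.
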(event `self.AttackPattern`
  (bind _mesh (`self.Mesh`))
  (`MeshComponent.SetScalarParameterValueOnMaterials` _mesh "isCharging" 1.0)
  (`KismetSystemLibrary.Delay` 0.6)
  (`MeshComponent.SetScalarParameterValueOnMaterials` _mesh "isCharging" 0.0)
  (set `self.canAttack` true)
  (`KismetSystemLibrary.Delay` 0.87)
  (set `self.canAttack` false)
  (`MeshComponent.SetScalarParameterValueOnMaterials` _mesh "isCharging" 1.0)
  (`KismetSystemLibrary.Delay` 1.2)
  (`MeshComponent.SetScalarParameterValueOnMaterials` _mesh "isCharging" 0.0)
  (set `self.canAttack` true)
  (`KismetSystemLibrary.Delay` 0.87)
  (set `self.canAttack` false))

(fn `UserConstructionScript`)