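; Monster AI character that roams, chases the player on sight and triggers an empty AttackPattern hook with a cooldown.
; PawnSensing drives the chase, with a retriggerable delay returning it to roaming, and damage briefly widens its vision.
; An overlap sphere toggles its health widget.
; Death registers it with the GameMode and hides it rather than destroying it, while reset events restore health and starting transform.
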(event `FacePlayer`
  (bind _playerref (`self.PlayerREF`))
  (bind (_returnvalue_roll _returnvalue_pitch _returnvalue_yaw) (`KismetMathLibrary.BreakRotator` (`KismetMathLibrary.RInterpTo` (`self.K2_GetActorRotation`) (`KismetMathLibrary.FindLookAtRotation` (`self.K2_GetActorLocation`) (`self.K2_GetActorLocation` _playerref)) (`GameplayStatics.GetWorldDeltaSeconds`) 15.0)))
  ;[1 0.6258 0.2725] Face the player (Optional)
  (if (`self.isDead`)
    _
    (elif (`KismetSystemLibrary.IsValid` _playerref)
      (`self.K2_SetActorRotation` (`KismetMathLibrary.MakeRotator` 0.0 0.0 _returnvalue_yaw))
      (`KismetSystemLibrary.Delay` 0.001)
      (`self.FacePlayer`))))

(event `self.K2_OnReset`
  ;[0.3182 0.6615 0.3667] Resetting Behaviour
  (set `self.health` (`self.maxHealth`))
  (`self.K2_SetActorTransform` (`self.OriginalTransform`))
  (`self.HealthWidgetSetup`)
  (if (`self.canRoam`)
    (`self.Roaming`)))

(event `ResetMonster`
  ;[0.3182 0.6615 0.3667] Resetting Behaviour
  (set `self.isDead` false)
  (set `self.health` (`self.maxHealth`))
  (`SceneComponent.SetVisibility` (`self.Mesh`) true false)
  (`self.K2_SetActorTransform` (`self.OriginalTransform`))
  (`self.HealthWidgetSetup`)
  (if (`self.canRoam`)
    (`self.Roaming`)))

(event `self.ReceiveBeginPlay`
  (set `self.OriginalTransform` (`self.GetTransform`))
  (`self.HealthWidgetSetup`)
  (set `self.PlayerREF` (`GameplayStatics.GetPlayerCharacter` 0))
  (if (`self.canRoam`)
    (`self.Roaming`)))

(event `UpdateHealthBar`
  ;[0.5938 0.01546 0.01546] Health Widget Stuff
  (bind _asenemy_minion_health_widget (cast `/Game/UI/Prompts/EnemyMinionHealthWidget` (`WidgetComponent.GetUserWidgetObject` (`self.Widget`))))
  (set `/Game/UI/Prompts/EnemyMinionHealthWidget.health` (`self.health`) _asenemy_minion_health_widget))

(event `HealthWidgetSetup`
  ;[0.5938 0.01546 0.01546] Health Widget Stuff
  (bind _asenemy_minion_health_widget (cast `/Game/UI/Prompts/EnemyMinionHealthWidget` (`WidgetComponent.GetUserWidgetObject` (`self.Widget`))))
  (set `/Game/UI/Prompts/EnemyMinionHealthWidget.health` (`self.health`) _asenemy_minion_health_widget)
  (set `/Game/UI/Prompts/EnemyMinionHealthWidget.maxHealth` (`self.maxHealth`) _asenemy_minion_health_widget))

(event `self.Sphere.OnComponentBeginOverlap`
  (params (OverlappedComponent :type "PrimitiveComponent Object Reference") (OtherActor :type "Actor Object Reference") (OtherComp :type "PrimitiveComponent Object Reference") (OtherBodyIndex :type Integer) (bFromSweep :type Boolean) (SweepResult :type "HitResult Structure (by ref)"))
  ;[0.5938 0.01546 0.01546] Health Widget Stuff
  (cast `/Game/ThirdPerson/Blueprints/BP_ThirdPersonCharacter` OtherActor)
  (`SceneComponent.SetHiddenInGame` (`self.Widget`) false false))

(event `Roaming`
  (bind _charactermovement (`self.CharacterMovement`))
  ;[0.25 0.1243 0.2416] Roaming Behaviour
  (if (`self.isDead`)
    _
    (elif (`self.isSeeingPlayer`)
      (set `CharacterMovementComponent.MaxWalkSpeed` (`self.MaxSpeed`) _charactermovement)
      (else
        (set `CharacterMovementComponent.MaxWalkSpeed` 100.0 _charactermovement)
        (`|AIMoveTo` self (`NavigationSystemV1.K2_GetRandomReachablePointInRadius` (`self.K2_GetActorLocation`) 2000.0 null null) null 75.0 true
          (:`OnSuccess`
            (`KismetSystemLibrary.Delay` 0.9)
            (`self.Roaming`)))))))

(event `self.Sphere.OnComponentEndOverlap`
  (params (OverlappedComponent :type "PrimitiveComponent Object Reference") (OtherActor :type "Actor Object Reference") (OtherComp :type "PrimitiveComponent Object Reference") (OtherBodyIndex :type Integer))
  ;[0.5938 0.01546 0.01546] Health Widget Stuff
  (cast `/Game/ThirdPerson/Blueprints/BP_ThirdPersonCharacter` OtherActor)
  (`SceneComponent.SetHiddenInGame` (`self.Widget`) true false))

(event `self.ReceiveAnyDamage`
  (params (Damage :type "Float (single-precision)") (DamageType :type "DamageType Object Reference") (InstigatedBy :type "Controller Object Reference") (DamageCauser :type "Actor Object Reference"))
  (bind _pawnsensing (`self.PawnSensing`))
  ;[0.1198 0.1198 0.1198] Damage and dying
  ;;[0.6042 0 0.01617 1 12] So the enemy notices player
  (`PawnSensingComponent.SetPeripheralVisionAngle` _pawnsensing 180.0)
  (bind _output_get (set `self.health` (- (`self.health`) Damage)))
  (`GameplayStatics.PlaySoundAtLocation` (`self.HitSound`) (`SceneComponent.K2_GetComponentLocation` (`self.Mesh`)) (struct) 1.0 1.0 0.0 null null null null)
  (`self.UpdateHealthBar`)
  (if (<= _output_get 0.0)
    (set `self.isDead` true)
    (`KismetSystemLibrary.Delay` 3.0)
    (bind _asbp_third_person_game_mode (cast `/Game/ThirdPerson/Blueprints/BP_ThirdPersonGameMode` (`GameplayStatics.GetGameMode`)))
    (`KismetArrayLibrary.Array_AddUnique` (`/Game/ThirdPerson/Blueprints/BP_ThirdPersonGameMode.KilledEnemiesStorage` _asbp_third_person_game_mode) self)
    ;;[0.1851 0.559 1 1 16] Hide until deletion
    (`SceneComponent.SetVisibility` (`self.Mesh`) false false)
    (`self.K2_SetActorTransform` (`KismetMathLibrary.MakeTransform` (0.0 0.0 0.0)))
    (else
      (`KismetSystemLibrary.Delay` 1.0)
      (`PawnSensingComponent.SetPeripheralVisionAngle` _pawnsensing 70.0))))

(event `self.PawnSensing.OnSeePawn`
  (params (Pawn :type "Pawn Object Reference"))
  ;[0.08333 0.01736 0.01736] Attack Pattern System
  (if (not (`self.isDead`))
    (set `self.isSeeingPlayer` true)
    (`|ExecutionSequence`
      (:`then_0`
        (set `CharacterMovementComponent.MaxWalkSpeed` (`self.MaxSpeed`) (`self.CharacterMovement`))
        (`self.FollowPlayer`))
      (:`then_1`
        (`KismetSystemLibrary.RetriggerableDelay` 0.6)
        (set `self.isSeeingPlayer` false)
        (if (`self.canRoam`)
          (`self.Roaming`))))))

(event `Drop Loot`
  (bind _returnvalue (`self.K2_GetActorLocation`))
  ;[1 1 1] Might Implement Loot Dropping for keys
  (bind _outhit (`KismetSystemLibrary.LineTraceSingle` _returnvalue (- _returnvalue (0.0 0.0 1000.0)) "TraceTypeQuery1" false (`|MakeArray` (`GameplayStatics.GetPlayerCharacter` 0) :!type "Actor Object Reference")))
  (`|SpawnActorFromClass` "/Game/ModularRuins/SpecialObjects/Openables/Keys/BP_Key.BP_Key_C" (`KismetMathLibrary.Conv_VectorToTransform` (`NavigationSystemV1.K2_GetRandomReachablePointInRadius` (`.Location` (`GameplayStatics.BreakHitResult` _outhit)) 100.0 null null)) "AdjustIfPossibleButDontSpawnIfColliding" "OverrideRootScale" null null))

(event `FollowPlayer`
  ;[0.08333 0.01736 0.01736] Attack Pattern System
  (if (and (not (`self.isDead`)) (`self.isSeeingPlayer`))
    (`|AIMoveTo` self (0.0 0.0 0.0) (`GameplayStatics.GetPlayerCharacter` 0) (`self.Acceptance Radius`) true
      (:`OnSuccess`
        (if (not (`self.inAttackPattern`))
          (set `self.inAttackPattern` true)
          (`self.AttackPattern`)
          (`KismetSystemLibrary.Delay` 5.0)
          (set `self.inAttackPattern` false))))))

(event `AttackPattern`
  ;[0.08333 0.01736 0.01736] Attack Pattern System
)

(fn `UserConstructionScript`)