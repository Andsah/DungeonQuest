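; Skeleton enemy that chases the player on sight, attacks at close range and can be killed.
; Pawn sensing triggers an AI MoveTo toward the player, and arrival fires the attack pattern component, gated by a cooldown flag.
; Taking damage briefly widens peripheral vision so the skeleton notices the player.
; At zero health it sets a dead flag, plays the death animation and destroys itself after a delay.
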(event `self.PawnSensing.OnSeePawn`
  (params (Pawn :type "Pawn Object Reference"))
  (set `self.isSeeingPlayer` true)
  (`self.FollowPlayer`))

(event `FollowPlayer`
  (if (and (not (`self.isDead`)) (`self.isSeeingPlayer`))
    (`|AIMoveTo` self (0.0 0.0 0.0) (`GameplayStatics.GetPlayerCharacter` 0) 75.0 true
      (:`OnSuccess`
        (if (not (`self.inAttackPattern`))
          (set `self.inAttackPattern` true)
          (`/Game/AI/Monsters/SkeletonComponentAttackPattern.SkeletonAttack` (`self.SkeletonComponentAttackPattern`))
          (`KismetSystemLibrary.Delay` 3.0)
          (set `self.inAttackPattern` false))))))

(event `self.ReceiveAnyDamage`
  (params (Damage :type "Float (single-precision)") (DamageType :type "DamageType Object Reference") (InstigatedBy :type "Controller Object Reference") (DamageCauser :type "Actor Object Reference"))
  (bind _pawnsensing (`self.PawnSensing`))
  ;[0.1198 0.1198 0.1198] Damage and dying
  ;;[0.6042 0 0.01617 1 12] So the enemy notices player
  (`PawnSensingComponent.SetPeripheralVisionAngle` _pawnsensing 180.0)
  (bind _output_get (set `self.health` (- (`self.health`) Damage)))
  (bind _returnvalue (<= _output_get 0.0))
  (if _returnvalue
    (set `self.isDead` _returnvalue)
    (`SkeletalMeshComponent.PlayAnimation` (`self.Mesh`) "/Game/AI/Monsters/Animations/Skeleton/Skeleton_Anim_SkeletonArmature_Skeleton_Death.Skeleton_Anim_SkeletonArmature_Skeleton_Death" false)
    (`KismetSystemLibrary.Delay` 3.0)
    (`self.K2_DestroyActor`)
    (else
      (`KismetSystemLibrary.Delay` 0.2)
      (`PawnSensingComponent.SetPeripheralVisionAngle` _pawnsensing 70.0))))

(fn `UserConstructionScript`)